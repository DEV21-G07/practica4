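; Door_Card_BP is a card-locked door that opens permanently when a player carrying at least one card walks into its trigger.
; On overlap it checks the first-person character for a card, consumes one and activates two steam effects.
; A timeline then slides the small door mesh from its closed to open position, and an Opened flag blocks any further triggering.
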(event `self.Trigger.OnComponentBeginOverlap`
  (params (OverlappedComponent :type "PrimitiveComponent Object Reference") (OtherActor :type "Actor Object Reference") (OtherComp :type "PrimitiveComponent Object Reference") (OtherBodyIndex :type Integer) (bFromSweep :type Boolean) (SweepResult :type "HitResult Structure (by ref)"))
  ;[1 1 1] Player overlaps with this door: check if player has at least 1 card to open door, if so, permantently open the door and substract cards
  (if (not (`self.Opened`))
    (bind _asfirst_person_character (cast `/Game/FirstPersonBP/Blueprints/FirstPersonCharacter` OtherActor))
    (if (`/Game/FirstPersonBP/Blueprints/FirstPersonCharacter.HasCard` _asfirst_person_character)
      (`/Game/FirstPersonBP/Blueprints/FirstPersonCharacter.DecreaseCards` _asfirst_person_character)
      (`ActorComponent.Activate` (`self.SteamDoor`) false)
      (`ActorComponent.Activate` (`self.SteamDoor2`) false)
      (bind (_direction _doorposition) (`Timeline|Timeline_0`)
        (:`Update`
          (`SceneComponent.K2_SetRelativeLocation` (`self.Door_Small_A`) (`KismetMathLibrary.VLerp` (`self.DoorClosed`) (`self.DoorOpen`) _doorposition) false false)
          (set `self.Opened` true))))))

(fn `UserConstructionScript`)